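; Game instance for the escape game, handling saves, level switching and top-level UI.
; A single "MainSave" slot stores the current level, written asynchronously and loaded when the main menu opens.
; SwitchLevel opens a LevelArray entry by index and overwrites the save with it.
; UI events create the menu, pause and in-game widgets, managing the cursor and pause state.
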(event Custom|SwitchLevel
  (params (WhichLevel :type Integer))
  (bind _levelarray (Variables|Default|GetLevelArray))
  (bind _output (Utilities|Array|Get(acopy) _levelarray WhichLevel))
  ;[1 1 1] SwitchLevel
  (if (and (< WhichLevel (Utilities|Array|Length (Variables|Default|GetLevelArray))) (>= WhichLevel 0))
    (Game|OpenLevel(byObjectReference) _output)
    (Variables|Default|SetCurrentLevel _output)
    (CallFunction|SaveGame true)))

(event Custom|Load_MainMenu
  ;[0.4417 0.6589 1] Menu UI
  (Game|SetGamePaused false)
  (Variables|Default|SetIsPaused false)
  (bind _returnvalue (UserInterface|CreateWidget "/Game/Game/UI/UWB_MainMenu.UWB_MainMenu_C"))
  (UserInterface|Viewport|AddtoViewport _returnvalue 0)
  (Variables|/Script/Engine.PlayerController|SetbShowMouseCursor (Game|GetPlayerController 0) true)
  (CallFunction|LoadGame))

(event Custom|Exit_Menu
  ;[0.4417 0.6589 1] Menu UI
  (Variables|/Script/Engine.PlayerController|SetbShowMouseCursor (Game|GetPlayerController 0) false))

(event Custom|SaveGame
  (params (OverwriteData :type Boolean))
  (bind _currentlevel (Variables|Default|GetCurrentLevel))
  ;[1 1 1] Save handler
  ;;[1 1 1] Saving
  (bind _returnvalue (SaveGame|DoesSaveGameExist "MainSave"))
  (if _returnvalue
    (if OverwriteData
      (bind _returnvalue_2 (SaveGame|CreateSaveGameObject "/Game/Game/Blueprints/Data/SG_SaveGameObject.SG_SaveGameObject_C" :!label _label))
      (bind _output_get (Variables|Default|SetSaveGameInstance _returnvalue_2))
      (if (Utilities|IsValidSoftObjectReference _currentlevel)
        (Variables|/Game/Game/Blueprints/Data/SG_SaveGameObject.SG_SaveGameObject_C|SetCurrentPlayerFloor _output_get _currentlevel)
        (|AsyncSaveGametoSlot _output_get 0 (Variables|/Game/Game/Blueprints/Data/SG_SaveGameObject.SG_SaveGameObject_C|GetSaveSlotName _output_get) (Variables|/Game/Game/Blueprints/Data/SG_SaveGameObject.SG_SaveGameObject_C|GetUserIndex _output_get))))
    (else
      (goto _label))))

(event Custom|LoadGame
  ;[1 1 1] Save handler
  ;;[1 1 1] Loading
  (bind (_savegame _bsuccess) (|AsyncLoadGamefromSlot "MainSave")
    (:Completed
      (if _bsuccess
        (bind _assg_save_game_object (Utilities|Casting|CastToSG_SaveGameObject _savegame))
        (Variables|Default|SetCurrentLevel (Variables|/Game/Game/Blueprints/Data/SG_SaveGameObject.SG_SaveGameObject_C|GetCurrentPlayerFloor _assg_save_game_object))
        (else
          (Development|PrintString "Couldnt Load saved game"))))))

(event Custom|DeleteSave
  ;[1 1 1] Save handler
  ;;[1 1 1] Deleting
  (SaveGame|DeleteGameinSlot "MainSave"))

(event Custom|TogglePauseUI
  (bind _returnvalue (Game|GetPlayerController 0))
  ;[0.4417 0.6589 1] Pause UI
  (if (Variables|Default|GetIsPaused)
    (CallFunction|ToggleGameUI true)
    (Variables|Default|SetIsPaused false)
    (Variables|/Script/Engine.PlayerController|SetbShowMouseCursor _returnvalue false)
    (Game|SetGamePaused false)
    (else
      (bind _returnvalue_2 (UserInterface|CreateWidget "/Game/Game/UI/UWB_Pause.UWB_Pause_C"))
      (UserInterface|Viewport|AddtoViewport _returnvalue_2 0)
      (Variables|Default|SetIsPaused true)
      (Variables|/Script/Engine.PlayerController|SetbShowMouseCursor _returnvalue true)
      (Game|SetGamePaused true))))

(event Custom|ToggleGameUI
  (params (Show? :type Boolean))
  ;[0.4417 0.6589 1] Game HUD
  (if Show?
    (bind _returnvalue (UserInterface|CreateWidget "/Game/Game/UI/UWB_InGame.UWB_InGame_C"))
    (UserInterface|Viewport|AddtoViewport _returnvalue 0)
    (Variables|/Script/Engine.PlayerController|SetbShowMouseCursor (Game|GetPlayerController 0) false)
    (Development|PrintString "turn on ui")
    (else
      (Viewport|RemoveAllWidgets))))