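; Player inventory component for an escape game, with fixed-size slots, item pickup and drop, and crafting.
; Slots store actor classes: pickup fills the first empty one, and dropping spawns the item ahead of the player.
; Queuing a second item triggers an order-independent match against GI_EscapeGame recipes by removing from an ingredient copy.
; Success empties used slots and spawns the output into inventory; failure clears the selection.
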(event Custom|ChangeInventorySize
  (params (NewSize :type Integer))
  (bind _inventory (Variables|Default|GetInventory))
  ;[1 1 1] Change inventory size
  (Utilities|Array|Resize _inventory NewSize)
  ;;[1 0.2333 0.9142] Debug
  (Development|PrintString (Utilities|String|Append "My new inventory size is:" (Utilities|String|ToString(Integer) (Utilities|Array|Length _inventory)))))

(event Custom|AddToInventory
  (params (Object :type Actor%20Object%20Reference) (DestroyPhysicalObject? :type Boolean))
  ;[1 1 1] Add item to inventory
  (Variables|Default|SetCouldAddItem false)
  (bind (_array_element _array_index) (Utilities|Array|ForEachLoopwithBreak (Variables|Default|GetInventory) :!label _label)
    (:LoopBody
      (if (not (Utilities|IsValidClass _array_element))
        (Variables|Default|SetCouldAddItem true)
        (Utilities|Array|SetArrayElem (Variables|Default|GetInventory) _array_index (Utilities|GetClass Object))
        (if DestroyPhysicalObject?
          (Actor|DestroyActor Object))
        (Development|PrintString (Utilities|String|Append "Added item to slot number " (Utilities|String|ToString(Integer) _array_index)))
        (goto _label Break)))
    (:Completed
      (if (not (Variables|Default|GetCouldAddItem))
        (Development|PrintString "Couldnt add item (replace with sound)")))))

(event Custom|RemoveFromInventory
  (params (InventorySlot :type Integer))
  (bind _returnvalue (Game|Player|GetPlayerPawn 0))
  (bind _rootcomponent (Variables|/Script/Engine.Actor|GetRootComponent _returnvalue))
  ;[1 1 1] Remove from inventory & drop item
  (Game|SpawnActorfromClass (Utilities|Array|Get(acopy) (Variables|Default|GetInventory) InventorySlot) (Math|Conversions|ToTransform(Vector) (+ (Transformation|GetWorldLocation _rootcomponent) (* (Math|Vector|GetForwardVector (Transformation|GetWorldRotation _rootcomponent)) 1.5e+02))) "Undefined" "MultiplyWithRoot" 0 0)
  (Utilities|Array|SetArrayElem (Variables|Default|GetInventory) InventorySlot 0))

(event Custom|AddItemToCraftList
  (bind _selectedinvspace (Variables|Default|GetSelectedInvSpace))
  (bind _inventory (Variables|Default|GetInventory))
  (bind _output (Utilities|Array|Get(acopy) _inventory _selectedinvspace))
  ;[1 1 1] Craft
  (if (Utilities|IsValidClass _output)
    (if (== (Utilities|Array|FindItem (Variables|Default|GetUsedInventorySlots) (Variables|Default|GetSelectedInvSpace)) -1)
      (Utilities|Array|Add (Variables|Default|GetCraftSlots) _output)
      (Utilities|Array|Add (Variables|Default|GetUsedInventorySlots) (Variables|Default|GetSelectedInvSpace))
      (if (>= (Utilities|Array|Length (Variables|Default|GetCraftSlots)) 2)
        (CallFunction|TryCraft)
        (else
          (Development|PrintString "Select another item")))
      (else
        (Development|PrintString "Slot already used")
        (Audio|PlaySound2D "/Game/Game/Audio/General/Wrong.Wrong" 1.0 1.0 0.0 0 0 :!label _label)))
    (else
      (Development|PrintString "Empty hand")
      (goto _label))))

(event Custom|TryCraft
  ;[1 1 1] Craft
  ;;[1 1 1] Check Recipes
  (bind _asgi_escape_game (Utilities|Casting|CastToGI_EscapeGame (Game|GetGameInstance)))
  (Development|PrintString "Enter try craft")
  (bind (_array_element _array_index) (Utilities|Array|ForEachLoopwithBreak (Variables|/Game/Game/Blueprints/Data/GI_EscapeGame.GI_EscapeGame_C|GetArrayRecipes _asgi_escape_game) :!label _label)
    (:LoopBody
      (Variables|Default|SetCanCraft true)
      (Development|PrintString "Iterating in recipes")
      (Variables|Default|SetRecipeRef _array_element)
      (Utilities|Array|Clear (Variables|Default|GetCopyIngredients))
      (if (== (Utilities|Array|Length (.ingredients (Utilities|Array|Get(acopy) (Variables|/Game/Game/Blueprints/Data/GI_EscapeGame.GI_EscapeGame_C|GetArrayRecipes _asgi_escape_game) _array_index))) (Utilities|Array|Length (Variables|Default|GetCraftSlots)))
        (bind _output_get (Variables|Default|SetCopyIngredients (.ingredients (Utilities|Array|Get(acopy) (Variables|/Game/Game/Blueprints/Data/GI_EscapeGame.GI_EscapeGame_C|GetArrayRecipes _asgi_escape_game) _array_index))))
        (for _array_element_2 (Variables|Default|GetCraftSlots)
          (if (!= (Utilities|Array|FindItem _output_get _array_element_2) -1)
            (Utilities|Array|RemoveIndex (Variables|Default|GetCopyIngredients) (Utilities|Array|FindItem _output_get _array_element_2))
            (if (== (Utilities|Array|Length (Variables|Default|GetCopyIngredients)) 0)
              (Variables|Default|SetCanCraft true)
              (goto _label Break)
              (else
                _)))
          (Variables|Default|SetCanCraft false))
        (if (Variables|Default|GetCanCraft)
          (goto _label Break))))
    (:Completed
      ;;;[1 0.6023 0.9006] Result
      (if (Variables|Default|GetCanCraft)
        (CallFunction|Craft)
        (else
          (Audio|PlaySound2D "/Game/Game/Audio/General/Wrong.Wrong" 1.0 1.0 0.0 0 0)
          (CallFunction|StopCrafting)
          (Development|PrintString "Couldnt craft"))))))

(event Custom|StopCrafting
  ;[1 1 1] Craft
  ;;[1 1 1] StopCraft
  (Utilities|Array|Clear (Variables|Default|GetCraftSlots))
  (Variables|Default|SetRecipeRef "")
  (Utilities|Array|Clear (Variables|Default|GetStoredIndexes))
  (Utilities|Array|Clear (Variables|Default|GetUsedInventorySlots)))

(event Custom|Craft
  (bind _returnvalue (Game|Player|GetPlayerPawn 0))
  (bind _reciperef (Variables|Default|GetRecipeRef))
  (bind _returnvalue_2 (Transformation|GetActorTransform _returnvalue))
  ;[1 1 1] Craft
  ;;[1 1 1] Craft item
  ;;;[1 1 1] Remove from inventory
  (for _array_element (Variables|Default|GetUsedInventorySlots)
    (Utilities|Array|SetArrayElem (Variables|Default|GetInventory) _array_element 0)
    (Development|PrintString "Remove element"))
  ;;;[1 1 1] Craft success
  (bind _returnvalue_3 (Game|SpawnActorfromClass (.output _reciperef) (Math|Transform|MakeTransform (Math|Vector|MakeVector (.x (.location _returnvalue_2)) (.y (.location _returnvalue_2)) (- (.z (.location _returnvalue_2)) -6e+01)) (.rotation _returnvalue_2) (.scale _returnvalue_2)) "AlwaysSpawn" "MultiplyWithRoot" 0 0))
  (CallFunction|AddtoInventory _returnvalue_3 true)
  (Audio|PlaySound2D (.sound _reciperef) 1.0 1.0 0.0 0 0)
  (CallFunction|StopCrafting)
  (Variables|Default|SetCanCraft true))

(event EventBeginPlay
  ;[1 1 1] Setup
  (CallFunction|ChangeInventorySize (Variables|Default|GetInventorySpace)))