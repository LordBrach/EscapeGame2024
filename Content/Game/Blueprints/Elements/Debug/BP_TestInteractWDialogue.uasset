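; Debug test actor for an interactable object that can play dialogue and show an outline.
; Interact only prints a test string.
; CallDialogue sends DialogueRef, if not empty, to the HUD_EscapeGame chatbox, using HasDialoguePlayed to fire only once.
; ToggleOutline switches custom depth rendering on the placeholder Cube mesh.
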(event EventBeginPlay)

(event Collision|EventActorBeginOverlap
  (params (OtherActor :type Actor%20Object%20Reference)))

(event EventTick
  (params (DeltaSeconds :type Float%20%28single-precision%29)))

(event EventInteract
  (Development|PrintString "Hello i am interactable object"))

(event EventCallDialogue
  (if (not (Variables|Default|GetHasDialoguePlayed))
    (if (not (Utilities|Array|IsEmpty (Variables|Default|GetDialogueRef)))
      (Variables|Default|SetHasDialoguePlayed true)
      (bind _ashud_escape_game (Utilities|Casting|CastToHUD_EscapeGame (HUD|GetHUD (Game|GetPlayerController 0))))
      (Default|CEUpdateChatbox _ashud_escape_game (Variables|Default|GetDialogueRef)))))

(event EventToggleOutline
  (params (OutlineValue :type Boolean))
  ;[1 1 1] Outline handler
  (Rendering|SetRenderCustomDepth (Variables|Default|GetCube) OutlineValue))

(fn ConstructionScript)