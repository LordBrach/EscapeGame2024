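; BP_TestNumpad is a debug interactable that tests the numpad code puzzle in the escape game.
; Interacting while unsolved toggles the numpad on HUD_EscapeGame, passing the correct code and itself as owner.
; A PositiveSignal event marks it solved, which blocks further interaction, and prints a success message.
; ToggleOutline switches custom depth rendering on the cube mesh for outlining.
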(event EventBeginPlay)

(event Collision|EventActorBeginOverlap
  (params (OtherActor :type Actor%20Object%20Reference)))

(event EventTick
  (params (DeltaSeconds :type Float%20%28single-precision%29)))

(event EventInteract
  (if (not (Variables|Default|GetSolved))
    (bind _ashud_escape_game (Utilities|Casting|CastToHUD_EscapeGame (HUD|GetHUD (Game|GetPlayerController 0))))
    (Default|ToggleNumpad _ashud_escape_game (Variables|Default|GetCode) self)))

(event EventPositiveSignal
  (Variables|Default|SetSolved true)
  (Development|PrintString "Good code !"))

(event EventToggleOutline
  (params (OutlineValue :type Boolean))
  ;[1 1 1] Outline handler
  (Rendering|SetRenderCustomDepth (Variables|Default|GetCube) OutlineValue))

(fn ConstructionScript)