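; Puzzle manager for the Level 03 rotating statues that unlocks a linked object when the statues are completed in the right order.
; On BeginPlay it binds to the correct and cancel events of every statue in its list.
; Each correct event appends a value to the player's answer, which is compared in order with the puzzle answer once lengths match.
; A mismatch or cancel resets all statue rotations and clears the answer.
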(event Custom|CheckCorrect
  (params (NewParam :type Integer))
  ;[1 1 1] Check if correct
  (Development|PrintString "Check Correct")
  (Utilities|Array|Add (Variables|Default|GetPlayerAnswer) NewParam)
  (Variables|Default|SetError? false)
  (if (== (Utilities|Array|Length (Variables|Default|GetPuzzleAnswer)) (Utilities|Array|Length (Variables|Default|GetPlayerAnswer)))
    (bind (_array_element _array_index) (Utilities|Array|ForEachLoopwithBreak (Variables|Default|GetPuzzleAnswer) :!label _label)
      (:LoopBody
        (if (not (== _array_element (Utilities|Array|Get(acopy) (Variables|Default|GetPlayerAnswer) _array_index)))
          (Variables|Default|SetError? true)
          (goto _label Break)))
      (:Completed
        (if (Variables|Default|GetError?)
          (CallFunction|ResetAll)
          (else
            (CallFunction|Solved)))))))

(event Custom|ResetAll
  (params (ID%20Statue :type Integer))
  ;[1 1 1] Reset
  (for _array_element (Variables|Default|GetStatues)
    (Default|ResetRotation _array_element)
    (Utilities|Array|Clear (Variables|Default|GetPlayerAnswer))))

(event Custom|Solved
  (bind _linkedobject (Variables|Default|GetLinkedObject))
  ;[1 1 1] Solved
  (Development|PrintString "Solved !")
  (Utilities|IsValid _linkedobject
    (:Is%20Valid
      (Default|Unlock _linkedobject))))

(event EventBeginPlay
  (for _array_element (Variables|Default|GetStatues)
    (EventDispatchers|BindEventtoCorrect! _array_element (delegate Custom|CheckCorrect))
    (EventDispatchers|BindEventtoCancel _array_element (delegate Custom|ResetAll))))

(fn ConstructionScript)