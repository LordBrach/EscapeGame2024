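; Interactable rotating statue for a puzzle, with a toggleable custom-depth outline and debug prints.
; When enabled, each interaction advances one of four 90-degree yaw states through a timeline-driven quaternion slerp with fading audio.
; Reaching the correct state marks it solved and calls Correct with the statue ID; interacting again while solved calls Cancel.
; ResetRotation clears the solved flag and animates back to the rotation and state saved at BeginPlay.
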(event Custom|Rotate
  (bind _statuemesh (Variables|Default|GetStatueMesh))
  (bind _relativerotation (Variables|/Script/Engine.SceneComponent|GetRelativeRotation _statuemesh))
  ;[1 1 1] Rotate
  (if (not (Variables|RotationStuff|GetIsRotating))
    (Variables|RotationStuff|SetIsRotating true)
    (if (>= (Variables|RotationStuff|GetRotateState) 3)
      (Variables|RotationStuff|SetRotateState 0)
      (else
        (Math|Integer|IncrementInt (Variables|RotationStuff|GetRotateState)
          (:%20%20
            (Development|PrintString (Utilities|String|Append "Rotate state: " (Utilities|String|ToString(Integer) (Variables|RotationStuff|GetRotateState))))))))
    (Audio|Components|Audio|Play (Variables|Default|GetAudio) 0.0)
    (Audio|Components|Audio|FadeOut (Variables|Default|GetAudio) 2.0 0.0 "Linear" :!class /Script/Engine.AudioComponent)
    (bind _statue (Timeline|Statue PlayFromStart)
      (:Update
        (Transformation|SetRelativeRotation (Variables|Default|GetStatueMesh) (Class|KismetMathLibrary|QuatRotator (Class|KismetMathLibrary|QuatSlerp (Math|Conversions|ToQuaternion(Rotator) (Math|Rotator|MakeRotator (.roll _relativerotation) (.pitch _relativerotation) (.yaw _relativerotation))) (Math|Conversions|ToQuaternion(Rotator) (Math|Rotator|MakeRotator (.roll _relativerotation) (.pitch _relativerotation) (Math|Conversions|ToFloat(Integer) (* (Variables|RotationStuff|GetRotateState) 90)))) _statue)) false false))
      (:Finished
        (Variables|RotationStuff|SetIsRotating false)))))

(event Custom|ResetRotation
  (bind _statuemesh (Variables|Default|GetStatueMesh))
  (bind _relativerotation (Variables|/Script/Engine.SceneComponent|GetRelativeRotation _statuemesh))
  ;[1 1 1] Reset
  (Variables|Default|SetSolved false)
  (Development|PrintString "Enter ResetRota")
  (Variables|RotationStuff|SetIsRotating true)
  (Audio|Components|Audio|Play (Variables|Default|GetAudio) 0.0)
  (Audio|Components|Audio|FadeOut (Variables|Default|GetAudio) 2.0 0.0 "Linear" :!class /Script/Engine.AudioComponent)
  (bind _statue (Timeline|Timeline PlayFromStart)
    (:Update
      (Transformation|SetRelativeRotation (Variables|Default|GetStatueMesh) (Class|KismetMathLibrary|QuatRotator (Class|KismetMathLibrary|QuatSlerp (Math|Conversions|ToQuaternion(Rotator) (Math|Rotator|MakeRotator (.roll _relativerotation) (.pitch _relativerotation) (.yaw _relativerotation))) (Math|Conversions|ToQuaternion(Rotator) (Variables|RotationStuff|GetOriginRotation)) _statue)) false false))
    (:Finished
      (Variables|RotationStuff|SetIsRotating false)
      (Variables|RotationStuff|SetRotateState (Variables|RotationStuff|GetOriginRotateState)))))

(event EventBeginPlay
  ;[1 1 1] Setup
  (Variables|RotationStuff|SetOriginRotation (Variables|/Script/Engine.SceneComponent|GetRelativeRotation (Variables|Default|GetStatueMesh)))
  (Variables|RotationStuff|SetOriginRotateState (Variables|RotationStuff|GetRotateState)))

(event EventInteract
  ;[1 1 1] Interact
  (if (Variables|Default|GetIsEnabled)
    (if (Variables|Default|GetSolved)
      (Default|CallCancel (Variables|Default|GetIDStatue)))
    (CallFunction|Rotate)
    (if (== (Variables|RotationStuff|GetRotateState) (Variables|RotationStuff|GetCorrectState))
      (Development|PrintString "Good rotation")
      (Variables|Default|SetSolved true)
      (Default|CallCorrect! (Variables|Default|GetIDStatue))
      (else
        (Variables|Default|SetSolved false)))))

(event EventToggleOutline
  (params (OutlineValue :type Boolean))
  ;[1 1 1] Outline handler
  (Rendering|SetRenderCustomDepth (Variables|Default|GetStatueMesh) OutlineValue))

(fn ConstructionScript)