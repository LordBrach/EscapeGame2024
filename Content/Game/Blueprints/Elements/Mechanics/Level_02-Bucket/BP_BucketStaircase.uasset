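; BP_BucketStaircase is an interactable bucket puzzle element that becomes a level exit in the escape game.
; Interact runs a three-state sequence: place the bucket, add ice cubes twice, then switch to LevelToGo through GI_EscapeGame.
; Placing the bucket sets ice cubes as the needed item, and the second ice addition clears the item requirement.
; ToggleOutline drives the mesh's custom depth for highlighting; step feedback is only printed strings.
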(event Custom|SwitchLevel
  ;[1 1 1] Switch level
  (bind _asgi_escape_game (Utilities|Casting|CastToGI_EscapeGame (Game|GetGameInstance)))
  (Default|SwitchLevel _asgi_escape_game (Variables|Default|GetLevelToGo)))

(event Custom|Interact%20add%20Bucket
  ;[1 1 1] Add bucket
  (Variables|Default|SetNeededItemType "/Game/Game/Blueprints/Elements/Mechanics/Level_02-Bucket/BP_TestIceCube.BP_TestIceCube_C")
  (Variables|Default|SetState 1)
  (Development|PrintString "Add bucket"))

(event Custom|Interact%20add%20IceCubes
  ;[1 1 1] Add ice
  (if (>= (Variables|Default|GetIceCounter) 1)
    (Variables|Default|SetState 2)
    (Variables|Default|SetNeedItem false)
    (Development|PrintString "Add ice 2")
    (else
      ;;[1 1 1] Step one
      (Math|Integer|IncrementInt (Variables|Default|GetIceCounter)
        (:%20%20
          (Development|PrintString "Add ice"))))))

(event EventBeginPlay)

(event EventInteract
  (if (== (Variables|Default|GetState) 2)
    (CallFunction|SwitchLevel)
    (elif (== (Variables|Default|GetState) 1)
      (CallFunction|InteractAddIceCubes)
      (else
        (CallFunction|InteractAddBucket)))))

(event EventToggleOutline
  (params (OutlineValue :type Boolean))
  ;[1 1 1] Outline handler
  (Rendering|SetRenderCustomDepth (Variables|Default|GetMesh) OutlineValue))

(fn ConstructionScript)