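; Rotation puzzle actor that spawns three puzzle pieces and signals when all are turned to the correct state.
; On BeginPlay it places each BP_PuzzlePiece at a top, left or right anchor with that anchor's material and a random starting rotation state.
; It binds to each piece's rotation update, rechecks all pieces against a hardcoded state of 1, and calls PuzzleSolved when every one matches.
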(event Custom|CheckRotations
  (Development|PrintString "Check Rotation")
  (Variables|Default|SetChecker true)
  (for _array_element (Variables|Default|GetPuzzlePieces)
    (if (not (== (Variables|/Game/Game/Blueprints/Elements/Mechanics/BP_PuzzlePiece.BP_PuzzlePiece_C|GetRotationState _array_element) 1))
      (Variables|Default|SetChecker false)))
  (if (Variables|Default|GetChecker)
    (Development|PrintString "Puzzle  solved !")
    (Default|CallPuzzleSolved)
    (else
      (Development|PrintString "Puzzle not solved"))))

(event EventBeginPlay
  (while (< (Variables|Default|GetIterator) 3)
    (bind (_location _material) (CallFunction|GetTransformPuzzlePiece))
    (bind _returnvalue (Game|SpawnActorfromClass "/Game/Game/Blueprints/Elements/Mechanics/BP_PuzzlePiece.BP_PuzzlePiece_C" (Math|Transform|MakeTransform _location (Transformation|GetSocketRotation (Variables|Default|GetBasePuzzleMesh) "None") "0.500000,0.500000,0.500000") "Undefined" "MultiplyWithRoot" 0 (Math|Random|RandomInteger 4) _material 1 "Interact" 0))
    (Utilities|Array|Add (Variables|Default|GetPuzzlePieces) _returnvalue)
    (Math|Integer|IncrementInt (Variables|Default|GetIterator)))
  (for _array_element (Variables|Default|GetPuzzlePieces)
    (EventDispatchers|BindEventtoUpdateRota _array_element (delegate Custom|CheckRotations))
    (Development|PrintString "Event bound")))

(fn ConstructionScript)

(fn GetTransformPuzzlePiece
  (bind _iterator (Variables|Default|GetIterator))
  (if (== _iterator 0)
    (return (Transformation|GetSocketLocation (Variables|Default|GetScene) "None") "/Game/Game/Art/ProgDebug/AnchorPuzzle/anchor_top_Mat.anchor_top_Mat")
    (elif (== _iterator 1)
      (return (Transformation|GetSocketLocation (Variables|Default|GetScene1) "None") "/Game/Game/Art/ProgDebug/AnchorPuzzle/anchor_left_Mat.anchor_left_Mat")
      (elif (== _iterator 2)
        (return (Transformation|GetSocketLocation (Variables|Default|GetScene2) "None") "/Game/Game/Art/ProgDebug/AnchorPuzzle/anchor_right_Mat.anchor_right_Mat")
        (else
          (Development|PrintString "False"))))))