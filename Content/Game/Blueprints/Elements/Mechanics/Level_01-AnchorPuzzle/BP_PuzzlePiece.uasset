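; BP_PuzzlePiece is an interactable piece, filed under the Level_01 anchor puzzle, that the player turns in quarter steps.
; Interact cycles RotationState through four values, and Rotate converts it to mesh yaw, then calls UpdateRota to signal the change.
; BeginPlay applies the piece's Texture material and starting rotation.
; ToggleOutline switches custom depth rendering on the mesh for highlighting.
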(event Custom|Rotate
  (Transformation|SetRelativeRotation (Variables|Default|GetMesh) (Math|Rotator|MakeRotator 0.0 0.0 (Math|Conversions|ToFloat(Integer) (* (Variables|Default|GetRotationState) 90))) false false)
  (Default|CallUpdateRota))

(event EventBeginPlay
  (Development|PrintString (Utilities|String|Append "Current state:" (Utilities|String|ToString(Integer) (Variables|Default|GetRotationState))))
  (Rendering|Material|SetMaterial (Variables|Default|GetMesh) 0 (Variables|Default|GetTexture))
  (CallFunction|Rotate))

(event EventInteract
  (Development|PrintString (Utilities|String|ToString(Integer) (Variables|Default|GetRotationState)))
  (if (< (Variables|Default|GetRotationState) 3)
    (Math|Integer|IncrementInt (Variables|Default|GetRotationState)
      (:%20%20
        _))
    (else
      (Variables|Default|SetRotationState 0)))
  (CallFunction|Rotate))

(event EventToggleOutline
  (params (OutlineValue :type Boolean))
  ;[1 1 1] Outline handler
  (Rendering|SetRenderCustomDepth (Variables|Default|GetMesh) OutlineValue))

(fn ConstructionScript)