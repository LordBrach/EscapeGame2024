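; Anchor rotation puzzle that rewards the player with a key item once all three pieces are correctly oriented.
; On BeginPlay it spawns three BP_PuzzlePiece actors at the left, right and top spots, each with an anchor material and a random incorrect rotation state.
; Each piece's UpdateRota event triggers a check of all pieces; the first full match calls PuzzleSolved and spawns BP_KeyBase at SpawnPosition.
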(event Custom|CheckRotations
  ;[1 1 1] Check puzzle
  (if (not (Variables|Default|GetIsSolved))
    (Development|PrintString "Check Rotation")
    (Variables|Default|SetChecker true)
    (for _array_element (Variables|Default|GetPuzzlePieces)
      (if (not (== (Variables|/Game/Game/Blueprints/Elements/Mechanics/Level_01-AnchorPuzzle/BP_PuzzlePiece.BP_PuzzlePiece_C|GetRotationState _array_element) 1))
        (Variables|Default|SetChecker false)))
    (if (Variables|Default|GetChecker)
      (Development|PrintString "Puzzle  solved !")
      (Default|CallPuzzleSolved)
      (Variables|Default|SetIsSolved true)
      (CallFunction|SpawnRopePiece)
      (else
        (Development|PrintString "Puzzle not solved")))))

(event Custom|SpawnRopePiece
  ;[1 1 1] Spawn the item
  (Game|SpawnActorfromClass "/Game/Game/Blueprints/Elements/BP_KeyBase.BP_KeyBase_C" (Transformation|GetWorldTransform (Variables|Default|GetSpawnPosition)) "AdjustIfPossibleButAlwaysSpawn" "MultiplyWithRoot" 0 "Interact" 0))

(event EventBeginPlay
  ;[1 1 1] Setup puzzle
  (while (< (Variables|Default|GetIterator) 3)
    (bind (_location _material) (CallFunction|GetTransformPuzzlePiece))
    (bind _returnvalue (Game|SpawnActorfromClass "/Game/Game/Blueprints/Elements/Mechanics/Level_01-AnchorPuzzle/BP_PuzzlePiece.BP_PuzzlePiece_C" (Math|Transform|MakeTransform _location (Transformation|GetSocketRotation (Variables|Default|GetBasePuzzleMesh) "None") "0.500000,0.500000,0.500000") "Undefined" "MultiplyWithRoot" 0 (Math|Random|RandomIntegerinRange 2 3) _material 1 "Interact" 0))
    (Utilities|Array|Add (Variables|Default|GetPuzzlePieces) _returnvalue)
    (Math|Integer|IncrementInt (Variables|Default|GetIterator)))
  ;[1 1 1] Bind to pieces
  (for _array_element (Variables|Default|GetPuzzlePieces)
    (EventDispatchers|BindEventtoUpdateRota _array_element (delegate Custom|CheckRotations))))

(fn ConstructionScript)

(fn GetTransformPuzzlePiece
  (bind _iterator (Variables|Default|GetIterator))
  (if (== _iterator 0)
    (return (Transformation|GetSocketLocation (Variables|Default|GetPuzzleSpotLeft) "None") "/Game/Game/Art/ProgDebug/AnchorPuzzle/anchor_top_Mat.anchor_top_Mat")
    (elif (== _iterator 1)
      (return (Transformation|GetSocketLocation (Variables|Default|GetPuzzleSpotRight) "None") "/Game/Game/Art/ProgDebug/AnchorPuzzle/anchor_left_Mat.anchor_left_Mat")
      (elif (== _iterator 2)
        (return (Transformation|GetSocketLocation (Variables|Default|GetPuzzleSpotTop) "None") "/Game/Game/Art/ProgDebug/AnchorPuzzle/anchor_right_Mat.anchor_right_Mat")
        (else
          (Development|PrintString "False"))))))