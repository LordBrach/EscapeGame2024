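; Pushable stool (tabouret) that slides once to a preset spot when the player interacts with it.
; BeginPlay caches the world transform of the WhereToMove component as the destination.
; Interact sets a one-shot active flag that Tick picks up to move the root there over DurationMove with MoveComponentTo.
; ToggleOutline drives the mesh's custom depth, only showing the outline while the stool can still be used.
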(event EventBeginPlay
  (bind _wheretomove (Variables|Default|GetWhereToMove))
  (Variables|Default|SetSavedDestination (Transformation|GetWorldLocation _wheretomove))
  (Variables|Default|SetSavedRotation (Transformation|GetWorldRotation _wheretomove)))

(event Collision|EventActorBeginOverlap
  (params (OtherActor :type Actor%20Object%20Reference)))

(event EventTick
  (params (DeltaSeconds :type Float%20%28single-precision%29))
  (if (Variables|Default|GetIsActive)
    (Components|MoveComponentTo (Variables|Default|GetDefaultSceneRoot) (Variables|Default|GetSavedDestination) (Variables|Default|GetSavedRotation) false false (Variables|Default|GetDurationMove) true)
    (Development|PrintString "Done")
    (Variables|Default|SetIsActive false)))

(event EventInteract
  (if (Variables|Default|GetDoOnce)
    (Development|PrintString "Hello i am a pushable object")
    (Variables|Default|SetIsActive true)
    (Variables|Default|SetDoOnce false)))

(event EventToggleOutline
  (params (OutlineValue :type Boolean))
  ;[1 1 1] Outline handler
  (if OutlineValue
    (if (Variables|Default|GetDoOnce) ; Just to not show the outline if the object cant be interacted with again
      (Rendering|SetRenderCustomDepth (Variables|Default|GetMesh) OutlineValue :!label _label))
    (else
      (goto _label))))

(fn ConstructionScript)