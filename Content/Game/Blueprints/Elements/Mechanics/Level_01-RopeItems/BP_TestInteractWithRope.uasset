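; BP_TestInteractWithRope is a test interactable for a rope mechanic, with debug prints standing in for the real actions.
; The first Interact sets the rope by enabling the actor and clearing NeedItem; once enabled, Interact pulls the rope a single time, guarded by Used.
; ToggleOutline switches custom depth rendering on the Cube mesh to show or hide an outline.
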(event EventBeginPlay)

(event Collision|EventActorBeginOverlap
  (params (OtherActor :type Actor%20Object%20Reference)))

(event EventTick
  (params (DeltaSeconds :type Float%20%28single-precision%29)))

(event EventInteract
  (if (Variables|Default|GetEnable)
    (if (not (Variables|Default|GetUsed))
      (Variables|Default|SetUsed true)
      (Development|PrintString "Pull Rope"))
    (else
      (Variables|Default|SetEnable true)
      (Development|PrintString "Set rope")
      (Variables|Default|SetNeedItem false))))

(event EventToggleOutline
  (params (OutlineValue :type Boolean))
  ;[1 1 1] Outline handler
  (Rendering|SetRenderCustomDepth (Variables|Default|GetCube) OutlineValue))

(fn ConstructionScript)