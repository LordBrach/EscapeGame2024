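; BP_RopePiece is an interactable rope-item actor for Level_01, still largely template placeholder logic.
; Interact only prints a debug message, and ToggleOutline switches custom depth rendering on the Cube mesh for highlighting.
; CallDialogue is empty, and a disconnected one-shot chain that would send DialogueRef to the HUD_EscapeGame chatbox never runs.
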(event EventBeginPlay)

(event Collision|EventActorBeginOverlap
  (params (OtherActor :type Actor%20Object%20Reference)))

(event EventTick
  (params (DeltaSeconds :type Float%20%28single-precision%29)))

(event EventInteract
  (Development|PrintString "Hello i am interactable object"))

(event EventCallDialogue)

(event EventToggleOutline
  (params (OutlineValue :type Boolean))
  ;[1 1 1] Outline handler
  (Rendering|SetRenderCustomDepth (Variables|Default|GetCube) OutlineValue))

(fn ConstructionScript)