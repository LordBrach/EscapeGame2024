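; BP_TestDoor is an interactable test door that swings 90 degrees open, optionally gated by locks.
; Interact opens it unless NeedLock is set, while InteractWithLock decrements NumberLocksNeeded and opens it at zero or below.
; OpenDoorTimeline, paced by DoorOpenSpeed, lerps the Pivot's world yaw from the mesh yaw saved at BeginPlay.
; ToggleOutline drives the mesh's custom depth, forcing it off when Used.
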(event Custom|OpenDoor
  (bind _pivot (Variables|Default|GetPivot))
  (bind _returnvalue (Transformation|GetWorldRotation _pivot))
  ;[1 1 1] Door opening
  (bind _dooropening (Timeline|OpenDoorTimeline Play)
    (:Update
      (Transformation|SetWorldRotation _pivot (Math|Rotator|MakeRotator (.roll _returnvalue) (.pitch _returnvalue) (Math|Float|Lerp (Variables|Default|GetSavedBaseRota) (+ (Variables|Default|GetSavedBaseRota) 9e+01) _dooropening)) false false))))

(event Custom|InteractWithLock
  ;[1 1 1] Interacts
  (bind _result (Math|Integer|DecrementInt (Variables|Default|GetNumberLocksNeeded))
    (:%20%20
      (if (<= _result 0)
        (Development|PrintString "Open door !")
        (CallFunction|OpenDoor)
        (else
          (Development|PrintString "Need to use the lock !"))))))

(event EventBeginPlay
  (Variables|Default|SetSavedBaseRota (.yaw (Transformation|GetWorldRotation (Variables|Default|GetMeshDoor))))
  (Components|Timeline|SetPlayRate (Variables|Default|GetOpenDoorTimeline) (Variables|Default|GetDoorOpenSpeed)))

(event EventInteract
  ;[1 1 1] Interacts
  (if (Variables|Default|GetNeedLock?)
    (Development|PrintString "need a lock !")
    (else
      (CallFunction|OpenDoor))))

(event EventToggleOutline
  (params (OutlineValue :type Boolean))
  (bind _meshdoor (Variables|Default|GetMeshDoor))
  ;[1 1 1] Outline handler
  (if (Variables|Default|GetUsed)
    (Rendering|SetRenderCustomDepth _meshdoor false)
    (else
      (Rendering|SetRenderCustomDepth _meshdoor OutlineValue))))

(fn ConstructionScript)