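; BP_LockBase is a lock actor that opens the doors sharing its ID when interacted with.
; On BeginPlay it gathers every BP_TestDoor with a matching ID into LinkedDoors.
; Interact prints a key-used message, calls InteractWithLock on each valid linked door and destroys the lock from inside that loop.
; ToggleOutline switches custom depth rendering on the placeholder Cube mesh for highlighting.
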(event EventBeginPlay
  ;[1 1 1] Find doors
  (bind _outactors (Actor|GetAllActorsOfClass "/Game/Game/Blueprints/Elements/BP_TestDoor.BP_TestDoor_C"))
  (bind _array_element (Utilities|Array|ForEachLoopwithBreak _outactors)
    (:LoopBody
      (if (== (Variables|Default|GetID) (Variables|/Game/Game/Blueprints/Elements/BP_TestDoor.BP_TestDoor_C|GetID _array_element))
        (Utilities|Array|Add (Variables|Default|GetLinkedDoors) _array_element)))))

(event EventInteract
  ;[1 1 1] Open linked doors
  (Development|PrintString "You used the key !")
  (for _array_element (Variables|Default|GetLinkedDoors)
    (if (Utilities|IsValid _array_element)
      (Default|InteractwithLock _array_element)
      (Actor|DestroyActor))))

(event EventToggleOutline
  (params (OutlineValue :type Boolean))
  ;[1 1 1] Outline handler
  (Rendering|SetRenderCustomDepth (Variables|Default|GetCube) OutlineValue))

(fn ConstructionScript)